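; Enemy spawner actor for the space shooter that periodically spawns enemies at random spawn points.
; A looping timer set on BeginPlay spawns at a random SpawnPoint-tagged component, picking between two enemy classes by a clamped random index bounded by the game mode's Level.
; Each enemy's destroy event decrements SpawnTime, but the running timer is never reset with the new value.
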(event Custom|Spawn
  (bind _enemy_spawned (CallFunction|SpawnEnemy))
  (EventDispatchers|BindEventtoOnEnemyDestroy _enemy_spawned (delegate Custom|EnemyDestroyed)))

(event Custom|EnemyDestroyed
  (Variables|Default|SetSpawnTime (- (Variables|Default|GetSpawnTime) 1.0)))

(event EventBeginPlay
  (Utilities|Time|SetTimerbyEvent (delegate Custom|Spawn) (Variables|Default|GetSpawnTime) true)
  (bind _asbp_ss_game_mode (Utilities|Casting|CastToBP_SS_GameMode (Game|GetGameMode)))
  (Variables|Default|Setm_GameMode _asbp_ss_game_mode))

(event Collision|EventActorBeginOverlap
  (params (OtherActor :type Actor%20Object%20Reference)))

(event EventTick
  (params (DeltaSeconds :type Float%20%28single-precision%29)))

(fn ConstructionScript)

(fn SpawnEnemy
  (bind _returnvalue (Actor|GetComponentsbyTag "/Script/Engine.SceneComponent" "SpawnPoint"))
  (bind _class (CallFunction|GetClasstoSpawn (Math|Random|RandomInteger (Variables|/Game/SpaceShooter/BP_SS_GameMode.BP_SS_GameMode_C|GetLevel (Variables|Default|Getm_GameMode)))))
  (bind _returnvalue_2 (Game|SpawnActorfromClass _class (Transformation|GetWorldTransform (Utilities|Array|Get(acopy) _returnvalue (Math|Random|RandomInteger (Utilities|Array|Length _returnvalue)))) "Undefined" "MultiplyWithRoot" 0 0))
  (bind _asbp_space_shooter_enemy_base (Utilities|Casting|CastToBP_SpaceShooterEnemyBase _returnvalue_2))
  (return _asbp_space_shooter_enemy_base))

(fn GetClasstoSpawn
  (params (Type :type Integer))
  (return (Utilities|Select :Index (Math|Integer|Clamp(Integer) Type 0 (- (Variables|Default|GetMaxNumEnemies) 1)) :Option%200 "/Game/SpaceShooter/Enemies/BP_SpaceShooterEnemyBase.BP_SpaceShooterEnemyBase_C" :Option%201 "/Game/SpaceShooter/Enemies/BP_SpaceShooterEnemyH.BP_SpaceShooterEnemyH_C")))