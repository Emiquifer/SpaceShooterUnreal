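; BP_SpaceShooterPawn is the player pawn for the space shooter, moving from Enhanced Input.
; BeginPlay adds its input mapping context, and the move action stores a 2D input that resets to zero when canceled or completed.
; Tick offsets the location along the right and forward vectors by that input, Speed and delta time, without sweeping.
; Firing is a placeholder that only prints a debug string.
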(event Input|EnhancedActionEvents|EnhancedInputActionBP_InputFire
  (params (ActionValue :type Boolean) (ElapsedSeconds :type Float%20%28double-precision%29) (TriggeredSeconds :type Float%20%28double-precision%29) (InputAction :type Input%20Action%20Object%20Reference :default "/Game/SpaceShooter/Inputs/BP_InputFire.BP_InputFire"))
  (:Triggered
    (Development|PrintString "Fire")))

(event Input|EnhancedActionEvents|EnhancedInputActionBP_InputMove
  (params (ActionValue :type Vector%202D%20Structure) (ElapsedSeconds :type Float%20%28double-precision%29) (TriggeredSeconds :type Float%20%28double-precision%29) (InputAction :type Input%20Action%20Object%20Reference :default "/Game/SpaceShooter/Inputs/BP_InputMove.BP_InputMove"))
  (:Triggered
    (Development|PrintString (Utilities|String|ToString(Vector2d) ActionValue))
    (Variables|Default|SetInput%20Saved ActionValue))
  (:Canceled
    (Variables|Default|SetInput%20Saved "" :!label _label))
  (:Completed
    (goto _label)))

(event EventBeginPlay
  (bind _asplayer_controller (Utilities|Casting|CastToPlayerController (Pawn|GetController)))
  (Utilities|IsValid (PlayerController|LocalPlayerSubsystems|GetEnhancedInputLocalPlayerSubsystem _asplayer_controller)
    (:Is%20Valid
      (Input|AddMappingContext (PlayerController|LocalPlayerSubsystems|GetEnhancedInputLocalPlayerSubsystem _asplayer_controller) "/Game/SpaceShooter/Inputs/BP_InputMapping.BP_InputMapping" 0 "(bIgnoreAllPressedKeysUntilRelease=True,bForceImmediately=False,bNotifyUserSettings=False)"))))

(event Collision|EventActorBeginOverlap
  (params (OtherActor :type Actor%20Object%20Reference)))

(event EventTick
  (params (DeltaSeconds :type Float%20%28single-precision%29))
  (bind _speed (Variables|Default|GetSpeed))
  (bind _input_saved (Variables|Default|GetInput%20Saved))
  (bind _returnvalue (* DeltaSeconds _speed))
  (Transformation|SetActorLocation (+ (+ (* (* (.x _input_saved) _returnvalue) (Transformation|GetActorRightVector)) (* (* _returnvalue (.y _input_saved)) (Transformation|GetActorForwardVector))) (Transformation|GetActorLocation)) false false))

(fn ConstructionScript)